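; BP_Metalball_Spawner is a stage hazard that knocks back the rabbit character when it touches the metal ball's collision.
; Overlaps from actors tagged PunchCollision are ignored; a BP_Rabbit instead receives OnPunchHit with a direction pointing away from this actor.
; The hit spawns a Niagara effect at the actor's location and briefly drops global time dilation for a hit-stop before restoring it.
; Despite the name, the graph contains no spawning of metal balls.
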(event OnComponentBeginOverlap(MetalballCollision)
  (params (OverlappedComponent :type Primitive%20Component%20Object%20Reference) (OtherActor :type Actor%20Object%20Reference) (OtherComp :type Primitive%20Component%20Object%20Reference) (OtherBodyIndex :type Integer) (bFromSweep :type Boolean) (SweepResult :type Hit%20Result%20Structure%20%28by%20ref%29))
  (if (not (Actor|ActorHasTag OtherActor "PunchCollision"))
    (bind _asbp_rabbit (Utilities|Casting|CastToBP_Rabbit OtherActor))
    (Default|OnPunchHit _asbp_rabbit (Math|Vector|Normalize (- (Transformation|GetActorLocation _asbp_rabbit) (Transformation|GetActorLocation))))
    (Niagara|SpawnSystematLocation "/Game/Basic_VFX/Niagara/NS_Basic_2.NS_Basic_2" (Transformation|GetActorLocation) "0, 0, 0" "3.000000,3.000000,3.000000")
    (Utilities|Time|SetGlobalTimeDilation 0.01)
    (Utilities|FlowControl|Delay 0.0)
    (Utilities|FlowControl|Delay 0.004)
    (Utilities|Time|SetGlobalTimeDilation 1.0)))

(event EventBeginPlay)

(event Collision|EventActorBeginOverlap
  (params (OtherActor :type Actor%20Object%20Reference)))

(event EventTick
  (params (DeltaSeconds :type Float%20%28single-precision%29)))

(fn ConstructionScript)